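; Enemy character Blueprint that chases the player and attacks on reaching them.
; From BeginPlay it loops AI MoveTo toward the player, plays an attack montage on arrival, then resumes the chase when that montage blends out.
; YouDied clears the CanMove flag that gates the chase, zeroes walk speed, plays the death montage and destroys the actor as it blends out.
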(event Custom|Attack
  ;[1 1 1] Attack the player
  (Animation|Montage|PlayMontage (Variables|Character|GetMesh) "/Game/Enemies/Mixamo/Animations/Attack_Montage.Attack_Montage"
    (:OnBlendOut
      (CallFunction|ChasePlayer))))

(event Custom|Chase%20Player
  ;[1 1 1] Chase the player
  (if (Variables|Default|GetCanMove)
    (AI|AIMoveTo self "0, 0, 0" (Game|GetPlayerCharacter 0) 1e+01 false
      (:OnSuccess
        (CallFunction|Attack)))))

(event Custom|You%20Died
  ;[1 1 1] Killing Enemy when hit
  (Variables|Default|SetCanMove false)
  (Variables|/Script/Engine.CharacterMovementComponent|SetMaxWalkSpeed (Variables|Character|GetCharacterMovement) 0.0)
  (Animation|Montage|PlayMontage (Variables|Character|GetMesh) "/Game/Enemies/Mixamo/Animations/ANM_Die_Montage.ANM_Die_Montage"
    (:OnBlendOut
      (Actor|DestroyActor))))

(event EventBeginPlay
  ;[1 1 1] To chase player
  (CallFunction|ChasePlayer))

(event Collision|EventActorBeginOverlap
  (params (OtherActor :type Actor%20Object%20Reference)))

(event EventTick
  (params (DeltaSeconds :type Float%20%28single-precision%29)))

(fn ConstructionScript)