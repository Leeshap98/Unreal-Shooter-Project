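; Zombie enemy character that chases and attacks the player, with 2D moan, attack and death sounds.
; PawnSensing spotting the player starts an AIMoveTo chase; reaching the player plays the attack montage, which resumes the chase on blend out.
; YouDied halts movement and plays the death montage, then updates the BP_ShooterGM progress bar and destroys the actor.
; No damage is applied in this graph.
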(event OnSeePawn(PawnSensing)
  (params (Pawn :type Pawn%20Object%20Reference))
  ;[1 1 1] To chase player
  (Utilities|Casting|CastToBP_FirstPersonCharacter Pawn)
  (CallFunction|ChasePlayer))

(event Custom|Attack
  ;[1 1 1] Attack the player
  (Audio|PlaySound2D "/Game/Enemies/Sounds/SC_ZombieAttack.SC_ZombieAttack" 1.0 1.0 0.0 0 0)
  (Animation|Montage|PlayMontage (Variables|Character|GetMesh) "/Game/Enemies/Mixamo/Animations/Attack_Montage.Attack_Montage"
    (:OnBlendOut
      (CallFunction|ChasePlayer))))

(event Custom|Chase%20Player
  ;[1 1 1] Chase the player
  (if (Variables|Default|GetCanMove)
    (bind _returnvalue (Audio|SpawnSound2D "/Game/Enemies/Sounds/SC_ZombieMoan.SC_ZombieMoan" 1.0 1.0 0.0 0))
    (bind _output_get (Variables|Default|SetWalkingSound _returnvalue))
    (Components|Activation|SetActive _output_get true false)
    (AI|AIMoveTo self "0, 0, 0" (Game|GetPlayerCharacter 0) 1e+01 false
      (:OnSuccess
        (CallFunction|Attack)))))

(event Custom|You%20Died
  ;[1 1 1] Enemy Killed
  (Variables|Default|SetCanMove false)
  (Variables|/Script/Engine.CharacterMovementComponent|SetMaxWalkSpeed (Variables|Character|GetCharacterMovement) 0.0)
  (Components|Activation|SetActive (Variables|Default|GetWalkingSound) false false)
  (Audio|SpawnSound2D "/Game/Enemies/Sounds/SC_ZombieDead.SC_ZombieDead" 1.0 1.0 0.0 0)
  (Animation|Montage|PlayMontage (Variables|Character|GetMesh) "/Game/Enemies/Mixamo/Animations/ANM_Die_Montage.ANM_Die_Montage"
    (:OnBlendOut
      (bind _asbp_shooter_gm (Utilities|Casting|CastToBP_ShooterGM (Game|GetGameMode)))
      (Default|UpdateProgressBar _asbp_shooter_gm)
      (Actor|DestroyActor))))

(event Collision|EventActorBeginOverlap
  (params (OtherActor :type Actor%20Object%20Reference)))

(event EventTick
  (params (DeltaSeconds :type Float%20%28single-precision%29)))

(fn ConstructionScript)