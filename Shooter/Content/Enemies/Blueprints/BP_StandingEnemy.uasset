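; BP_StandingEnemy is a zombie enemy with chase, attack and death events, and it stays idle on BeginPlay.
; ChasePlayer, gated by CanMove, starts a moan sound and uses AI MoveTo toward the player, calling Attack on success.
; Attack plays a sound and montage, then resumes the chase on blend out.
; YouDied plays death sound and animation, then destroys the actor immediately.
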(event Custom|Attack
  ;[1 1 1] Attack the player
  (Audio|PlaySound2D "/Game/Enemies/Sounds/SC_ZombieAttack.SC_ZombieAttack" 1.0 1.0 0.0 0 0)
  (Animation|Montage|PlayMontage (Variables|Character|GetMesh) "/Game/Enemies/Mixamo/Animations/Attack_Montage.Attack_Montage"
    (:OnBlendOut
      (CallFunction|ChasePlayer))))

(event Custom|Chase%20Player
  ;[1 1 1] Chase the player
  (if (Variables|Default|GetCanMove)
    (bind _returnvalue (Audio|SpawnSound2D "/Game/Enemies/Sounds/SC_ZombieMoan.SC_ZombieMoan" 1.0 1.0 0.0 0))
    (bind _output_get (Variables|Default|SetWalkingSound _returnvalue))
    (Components|Activation|SetActive _output_get true false)
    (AI|AIMoveTo self "0, 0, 0" (Game|GetPlayerCharacter 0) 1e+01 false
      (:OnSuccess
        (CallFunction|Attack)))))

(event Custom|You%20Died
  ;[1 1 1] Enemy Killed
  (Audio|SpawnSound2D "/Game/Enemies/Sounds/SC_ZombieDead.SC_ZombieDead" 1.0 1.0 0.0 0)
  (Components|Animation|PlayAnimation (Variables|Character|GetMesh) "/Game/Enemies/Mixamo/Animations/ANM_Die_Montage.ANM_Die_Montage" false)
  (Actor|DestroyActor))

(event EventBeginPlay
  ;[1 1 1] To chase player
)

(event Collision|EventActorBeginOverlap
  (params (OtherActor :type Actor%20Object%20Reference)))

(event EventTick
  (params (DeltaSeconds :type Float%20%28single-precision%29)))

(fn ConstructionScript)