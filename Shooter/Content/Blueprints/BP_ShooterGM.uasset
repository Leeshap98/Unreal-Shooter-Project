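; Shooter game mode that spawns the level's enemies at BeginPlay and tracks a running enemy count on the HUD progress bar.
; Standing enemies spawn immobile at random positions within fixed bounds, while walking enemies spawn movable at random reachable nav points around GLZone.
; BeginPlay totals both counts as MaxEnemies, then polls until the player character's HUD is valid and zeroes the bar.
; Each UpdateProgressBar call increments the count and sets the bar to its fraction of MaxEnemies.
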(event Custom|Spawn%20Enemies%20is%20GL_Zone
  ;[1 1 1] Spawning Walking Enemies
  (Utilities|FlowControl|ForLoopwithBreak 0 (Math|Float|Truncate (- (Variables|Default|GetWalkingEnemyCount) 1.0))
    (:LoopBody
      (bind _returnvalue (Game|SpawnActorfromClass "/Game/Enemies/Blueprints/BP_Enemy.BP_Enemy_C" (Math|Transform|MakeTransform (.RandomLocation (AI|Navigation|GetRandomReachablePointinRadius (Variables|Default|GetGL_Zone) 5.0 0 0)) "0, 0, 0" "1.000000,1.000000,1.000000") "Undefined" "MultiplyWithRoot" 0 0))
      (Utilities|IsValid _returnvalue
        (:Is%20Valid
          (Variables|/Game/Enemies/Blueprints/BP_Enemy.BP_Enemy_C|SetCanMove _returnvalue true)
          (Development|PrintString "1" true true "(R=0.978040,G=1.000000,B=0.000000,A=1.000000)" 12.0))))))

(event Custom|Spawn%20Standing%20Zombies
  ;[1 1 1] Spawning Standing Enemies
  (Utilities|FlowControl|ForLoopwithBreak 0 (Math|Float|Truncate (- (Variables|Default|GetStandingEnemyCount) 1.0))
    (:LoopBody
      (bind _returnvalue (Game|SpawnActorfromClass "/Game/Enemies/Blueprints/BP_Enemy.BP_Enemy_C" (Math|Transform|MakeTransform (Math|Vector|MakeVector (Math|Random|RandomFloatinRange 8e+01 4.26e+03) (Math|Random|RandomFloatinRange 0.0 5.06e+03) 75.0) "0, 0, 0" "1.000000,1.000000,1.000000") "Undefined" "MultiplyWithRoot" 0 0))
      (Utilities|IsValid _returnvalue
        (:Is%20Valid
          (Variables|/Game/Enemies/Blueprints/BP_Enemy.BP_Enemy_C|SetCanMove _returnvalue false)
          (Development|PrintString "2" true true "(R=0.000000,G=0.660000,B=1.000000,A=1.000000)" 12.0))))))

(event Custom|Update%20Progress%20Bar
  (bind _max_enemies (Variables|Default|GetMax%20Enemies))
  ;[1 1 1] Action
  (bind _output_get (Variables|Default|SetTotal%20Enemies%20Count (+ (Variables|Default|GetTotal%20Enemies%20Count) 1.0)))
  (Progress|SetPercent (Variables|/Game/Widgets/W_HUD.W_HUD_C|GetProgressBar_LP (Variables|Default|GetHUD)) (/ _output_get _max_enemies))
  (Development|PrintString (Utilities|String|Append "MaxEnemies" (Utilities|String|ToString(Float) _max_enemies) "Total Enemies" (Utilities|String|ToString(Float) _output_get))))

(event EventBeginPlay
  ;[1 1 1] Action
  (Utilities|FlowControl|Sequence
    (:then_0
      (CallFunction|SpawnStandingZombies))
    (:then_1
      (CallFunction|SpawnEnemiesIsGLZone))
    (:then_2
      (Variables|Default|SetMax%20Enemies (+ (Variables|Default|GetStandingEnemyCount) (Variables|Default|GetWalkingEnemyCount))))
    (:then_3
      (bind _asbp_first_person_character (Utilities|Casting|CastToBP_FirstPersonCharacter (Game|GetPlayerCharacter 0)))
      (Utilities|IsValid (Variables|/Game/FirstPerson/Blueprints/BP_FirstPersonCharacter.BP_FirstPersonCharacter_C|GetHUD%20UI _asbp_first_person_character) :!label _label
        (:Is%20Valid
          (bind _output_get (Variables|Default|SetHUD (Variables|/Game/FirstPerson/Blueprints/BP_FirstPersonCharacter.BP_FirstPersonCharacter_C|GetHUD%20UI _asbp_first_person_character)))
          (Progress|SetPercent (Variables|/Game/Widgets/W_HUD.W_HUD_C|GetProgressBar_LP _output_get) 0.0))
        (:Is%20Not%20Valid
          (Utilities|FlowControl|Delay 0.2)
          (goto _label))))))

(event EventTick
  (params (DeltaSeconds :type Float%20%28single-precision%29)))

(fn ConstructionScript)